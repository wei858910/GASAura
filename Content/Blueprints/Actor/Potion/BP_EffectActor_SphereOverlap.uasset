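; Potion effect actor that passes sphere begin-overlaps to OnOverlap and animates its mesh as a floating pickup.
; FloatctorEvent plays an initial drop timeline that moves the mesh's relative Z, then starts FlaotMesh, which drives a height offset and adds yaw spin each update.
; OnEndOverlap is left unwired, so ending an overlap does nothing here.
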(event `self.Sphere.OnComponentBeginOverlap`
  (params (OverlappedComponent :type "PrimitiveComponent Object Reference") (OtherActor :type "Actor Object Reference") (OtherComp :type "PrimitiveComponent Object Reference") (OtherBodyIndex :type Integer) (bFromSweep :type Boolean) (SweepResult :type "HitResult Structure (by ref)"))
  (`self.OnOverlap` OtherActor))

(event `self.Sphere.OnComponentEndOverlap`
  (params (OverlappedComponent :type "PrimitiveComponent Object Reference") (OtherActor :type "Actor Object Reference") (OtherComp :type "PrimitiveComponent Object Reference") (OtherBodyIndex :type Integer)))

(event `self.FloatctorEvent`
  (bind (_direction _alphaz) (`Timeline|刚开始掉落` :!via `PlayFromStart`)
    (:`Update`
      (`SceneComponent.K2_SetRelativeLocation` (`self.StaticMesh`) (`KismetMathLibrary.MakeVector` 0.0 0.0 (* _alphaz 30.0)) false false))
    (:`Finished`
      (bind (_direction_2 _alphabase) (`Timeline|FlaotMesh` :!via `PlayFromStart`)
        (:`Update`
          (`SceneComponent.K2_SetRelativeLocation` (`self.StaticMesh`) (`KismetMathLibrary.MakeVector` 0.0 0.0 (* _alphabase 16.0)) false false)
          (`SceneComponent.K2_AddRelativeRotation` (`self.StaticMesh`) (`KismetMathLibrary.MakeRotator` 0.0 0.0 0.2) false false))))))

(fn `UserConstructionScript`)