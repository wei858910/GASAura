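; BP_FlamePillar is a flame pillar actor that makes its light flicker with randomized intensity.
; BeginPlay starts a looping timer, apparently driving ExcuteSetIntersity, which rolls a random intensity multiplier and a coin flip between two timeline curves.
; The event restarts the flame timeline, whose updates set FileLight intensity from the chosen curve, base intensity and random multiplier.
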(event `self.ReceiveBeginPlay`
  (`KismetSystemLibrary.K2_SetTimerDelegate` (`|CreateDelegate` :!event `ExcuteSetIntersity`) 2.0 true))

(event `ExcuteSetIntersity`
  (bind _minlinghtintensity (`self.MinLinghtIntensity`))
  (bind _maxlinghtintensity (`self.MaxLinghtIntensity`))
  (bind _returnvalue (`KismetMathLibrary.RandomFloatInRange` _minlinghtintensity _maxlinghtintensity))
  (set `self.LinghtIntensityRadio` _returnvalue)
  (set `self.bIsOverHalf` (> _returnvalue (/ (+ _minlinghtintensity _maxlinghtintensity) 2.0)))
  (`|ExecutionSequence`
    (:`then_0`
      (bind (_direction _flameintersty_1 _flameintersty_2) (`Timeline|FlameIntenstyTimeline_1` :!via `Stop` :!label _label)
        (:`Update`
          (`LightComponent.SetIntensity` (`self.FileLight`) (* (* (`KismetMathLibrary.SelectFloat` _flameintersty_1 _flameintersty_2 (`self.bIsOverHalf`)) (`self.LinghtIntensityBase`)) (`self.LinghtIntensityRadio`))))))
    (:`then_1`
      (goto _label :!via `PlayFromStart`))))

(fn `UserConstructionScript`)