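; GA_MeleeAttack is the enemy melee attack gameplay ability, turning the avatar toward its combat target and playing a random tagged attack montage.
; A gameplay event matching the montage's socket tag triggers a small radius check at that combat socket, damaging live non-friendly actors found there.
; On any hit it fires the MeleeImpact gameplay cue with the montage tag, and the ability ends after the strike or montage end.
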(event `self.K2_ActivateAbility`
  (bind _returnvalue (`self.GetAvatarActorFromActorInfo`))
  (bind _returnvalue_2 (`self.GetAvatarActorFromActorInfo`))
  (`self.Init`)
  ;[1 1 1] 面向玩家
  (bind _returnvalue_3 (message `CombatInterface.GetCombatTarget` _returnvalue_2))
  (bind _ascombat_interface (cast `CombatInterface` _returnvalue_2)
    (:`then`
      (`/Engine/EditorBlueprintResources/StandardMacros.IsValid` _returnvalue_3
        (:`Is Valid`
          (`CombatInterface.SetFaceingTargetLoc` _ascombat_interface (`Actor.K2_GetActorLocation` _returnvalue_3))
          (bind _returnvalue_4 (message `CombatInterface.GetAttackMontages` (`self.GetAvatarActorFromActorInfo`)))
          (bind _output_get (set `self.SlecetedMontage` (`self.GetRandomTaggedMontage` _returnvalue_4)))
          (`AbilityTask_PlayMontageAndWait.CreatePlayMontageAndWaitProxy` "None" (break `TaggedMontage` _output_get) 1.0 "None" false
            (:`then`
              (`AbilityTask_WaitGameplayEvent.WaitGameplayEvent` (`.SocketTag` (break `TaggedMontage` _output_get)) null
                (:`EventReceived`
                  (bind _returnvalue_5 (`CombatInterface.GetCombatSocktLocation` _ascombat_interface (`.SocketTag` (break `TaggedMontage` _output_get))))
                  (bind _outoverlappingactors (`AuraAbilitySystemBPLibary.GetLivePlayersWithRadius` _returnvalue (`|MakeArray` _returnvalue) _returnvalue_5 66.0))
                  (`|ExecutionSequence`
                    (:`then_1`
                      (for _array_element _outoverlappingactors
                        (if (`AuraAbilitySystemBPLibary.IsNotFriend` _array_element (`self.GetAvatarActorFromActorInfo`) "Enemy")
                          (`self.CauseDamage` _array_element)
                          (set `self.HasHitAttack` true)))
                      (if (`self.HasHitAttack`)
                        (`self.K2_ExecuteGameplayCueWithParams` (struct :`TagName` "GameplayCue.MeleeImpact") (`AbilitySystemBlueprintLibrary.MakeGameplayCueParameters` 0.0 0.0 (struct) (struct) (struct) (`BlueprintGameplayTagLibrary.MakeGameplayTagContainerFromTag` (`.MontageTag` (break `TaggedMontage` _output_get))) (struct) _returnvalue_5 (0.0 0.0 0.0) null (`self.GetAvatarActorFromActorInfo`) _returnvalue_3)))
                      (`self.K2_EndAbility`))))))
            (:`OnCompleted`
              (`self.K2_EndAbility` :!label _label))
            (:`OnInterrupted`
              (goto _label))
            (:`OnCancelled`
              (goto _label))))
        (:`Is Not Valid`
          (`self.K2_EndAbility` :!label _label_2))))
    (:`CastFailed`
      (goto _label_2))))

(fn `Init`
  (set `self.HasHitAttack` false))