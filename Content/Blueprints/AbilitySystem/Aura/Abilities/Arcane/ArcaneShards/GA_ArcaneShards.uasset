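; GA_ArcaneShards is a targeted gameplay ability that spawns a series of arcane shard cues on the ground.
; On activation it shows a magic circle, ensures a reusable BP_PointCollection exists, then waits for input.
; The press moves the collection to the cursor hit, gets randomly rotated ground points, hides the circle and plays the cast montage.
; A looping timer then fires a GameplayCue and debug sphere per point; no damage is applied here.
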(event `self.K2_ActivateAbility`
  (bind _returnvalue (`self.GetAvatarActorFromActorInfo`))
  (`|ExecutionSequence`
    (:`then_0`
      (if (`KismetSystemLibrary.DoesImplementInterface` _returnvalue "/Script/Aura_Learn.CombatInterface")
        (message `PlayerInterface.ShowMagicCricle` _returnvalue null)
        (`self.CheckPointComponent`)
        (else
          (`self.K2_CancelAbility`))))
    (:`then_1`
      (`AbilityTask_WaitInputPress.WaitInputPress` false
        (:`OnPress`
          (bind (_asynctaskproxy _datahandle) (`TargetDataUnderMouse.CreateTargetDataUnderMouse`)
            (:`ValidData`
              (bind (_returnvalue_bblockinghit _returnvalue_binitialoverlap _returnvalue_time _returnvalue_distance _returnvalue_location _returnvalue_impactpoint) (`GameplayStatics.BreakHitResult` (`AbilitySystemBlueprintLibrary.GetHitResultFromTargetData` _datahandle)))
              (`Actor.K2_SetActorLocation` (`self.SpawnPoints`) _returnvalue_impactpoint false false)
              (set `self.PointsArray` (`PointCollection.GetGroundPoints` (`self.SpawnPoints`) _returnvalue_impactpoint (`self.Num Points`) (`KismetMathLibrary.RandomFloatInRange` 0.0 360.0)))
              (set `self.PointIndex` 0)
              (message `CombatInterface.SetFaceingTargetLoc` (`self.GetAvatarActorFromActorInfo`) _returnvalue_location)
              (message `PlayerInterface.HideMagicCricle` (`self.GetAvatarActorFromActorInfo`))
              (`AbilityTask_PlayMontageAndWait.CreatePlayMontageAndWaitProxy` "None" "/Game/Assets/Characters/Aura/Animations/Abilities/AM_Cast_ArcaneShards_Short.AM_Cast_ArcaneShards_Short" 1.0 "None" false
                (:`OnCompleted`
                  _)
                (:`OnBlendOut`
                  _)
                (:`OnInterrupted`
                  _))
              (bind _returnvalue_2 (`KismetSystemLibrary.K2_SetTimerDelegate` (delegate `SpawnShard`) (`self.SpawnDelta`) true))
              (set `self.SpawnShardHandl` _returnvalue_2)
              (`self.SpawnShard`))))))))

(event `SpawnShard`
  (if (< (`self.PointIndex`) (`self.Num Points`))
    (bind _output_get (set `self.SpawnLocation` (`SceneComponent.K2_GetComponentLocation` (`|GetArrayItem` (`self.PointsArray`) (`self.PointIndex`)))))
    (`KismetSystemLibrary.DrawDebugSphere` _output_get 20.0 8 (struct :`R` 1.0 :`G` 0.076088 :`A` 1.0) 10.0 2.0)
    (`/Engine/EditorBlueprintResources/StandardMacros.IncrementInt` (`self.PointIndex`)
      (:`  `
        (`self.K2_ExecuteGameplayCueWithParams` (struct :`TagName` "GameplayCue.ArcaneShards") (`AbilitySystemBlueprintLibrary.MakeGameplayCueParameters` 0.0 0.0 (struct) (struct) (struct) (struct) (struct) (`self.SpawnLocation`)))))
    (else
      (`KismetSystemLibrary.K2_ClearAndInvalidateTimerHandle` (`self.SpawnShardHandl`))
      (`KismetSystemLibrary.Delay` 0.2)
      (`self.K2_EndAbility`))))

(fn `CheckPointComponent`
  (`self.SpawnPoints`
    (:`then`)
    (:`else`
      (bind _returnvalue (`|SpawnActorFromClass` "/Game/Blueprints/AbilitySystem/Aura/Abilities/Arcane/ArcaneShards/BP_PointCollection.BP_PointCollection_C" (`KismetMathLibrary.MakeTransform` (`Actor.K2_GetActorLocation` (`self.GetAvatarActorFromActorInfo`))) "AlwaysSpawn" "MultiplyWithRoot" null null))
      (set `self.SpawnPoints` _returnvalue))))