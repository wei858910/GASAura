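; GA_ListenForEvent is a passive startup gameplay ability for Aura that turns incoming Attributes gameplay events into attribute effects on its owner.
; On activation it waits for events under the Attributes tag, accepting child tags.
; Each event builds a spec from EventBasedEffectClass, using the event's tag and magnitude as a SetByCaller value, and applies it to self.
; Debug strings print on activation and on each received event tag, and the graph never calls EndAbility.
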(event `self.K2_ActivateAbility`
  (bind _returnvalue (`self.GetAbilitySystemComponentFromActorInfo`))
  (`KismetSystemLibrary.PrintString` "Active Listen")
  (bind (_asynctaskproxy _payload) (`AbilityTask_WaitGameplayEvent.WaitGameplayEvent` (struct :`TagName` "Attributes") null false false)
    (:`EventReceived`
      (bind (_eventtag _instigator _target _optionalobject _optionalobject2 _contexthandle _instigatortags _targettags _eventmagnitude) (break `GameplayEventData` _payload))
      (`KismetSystemLibrary.PrintString` (`BlueprintGameplayTagLibrary.GetDebugStringFromGameplayTag` _eventtag) true true (struct :`G` 0.66 :`B` 1.0 :`A` 1.0) 10.0)
      (bind _returnvalue_2 (`AbilitySystemBlueprintLibrary.AssignTagSetByCallerMagnitude` (`AbilitySystemComponent.MakeOutgoingSpec` _returnvalue (`self.EventBasedEffectClass`) 1.0 (`AbilitySystemComponent.MakeEffectContext` _returnvalue)) _eventtag _eventmagnitude))
      (`AbilitySystemComponent.BP_ApplyGameplayEffectSpecToSelf` (`self.GetAbilitySystemComponentFromActorInfo`) _returnvalue_2))))