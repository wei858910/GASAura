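; Fireball projectile for the Fire Blast ability that flies outward, returns to its instigator and explodes on arrival.
; LaunchFire drives a timeline lerp from the spawn point to an apex along its forward vector.
; A looping timer then homes it toward the instigator's current position in fixed steps.
; Within range, it calls OnHit, applies radial damage with outward knockback to nearby live players except the instigator, and destroys itself.
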(event `self.LaunchFire`
  (`self.SetApexLocation`)
  (bind (_direction _outalpha) (`Timeline|时间轴` :!via `PlayFromStart`)
    (:`Update`
      (`self.K2_SetActorLocation` (`KismetMathLibrary.VLerp` (`self.BeginLocation`) (`self.ApexLocation`) _outalpha)))
    (:`Finished`
      (`self.BackToOnwer`))))

(event `self.BackToOnwer`
  (bind _returnvalue (`KismetSystemLibrary.K2_SetTimerDelegate` (delegate `执行回归`) 0.03 true))
  (set `self.执行回归事件` _returnvalue))

(event `执行回归`
  (bind _instigator (`self.Instigator`))
  (bind _returnvalue (- (`self.K2_GetActorLocation` _instigator) (`self.K2_GetActorLocation`)))
  (`/Engine/EditorBlueprintResources/StandardMacros.IsValid` _instigator
    (:`Is Valid`
      (if (<= (`KismetMathLibrary.VSize` _returnvalue) 188.0)
        (`KismetSystemLibrary.K2_ClearAndInvalidateTimerHandle` (`self.执行回归事件`))
        (`self.OnHit`)
        (bind _outoverlappingactors (`self.PureMakeDamageParam`))
        (for _array_element _outoverlappingactors
          (`self.ApplyDamageToTarget` _array_element))
        (`self.K2_DestroyActor`)
        (else
          (`self.K2_AddActorWorldOffset` (* (`KismetMathLibrary.Normal` _returnvalue) 40.0)))))))

(fn `ApplyDamageToTarget`
  (params (DamageTarget :type "Actor Object Reference"))
  (bind _explosiondamageparams (`self.ExplosionDamageParams`))
  (`AuraAbilitySystemBPLibary.SetDamageParamsKnockback` _explosiondamageparams (- (`self.K2_GetActorLocation` DamageTarget) (`self.K2_GetActorLocation`)) 666.0)
  (`AuraAbilitySystemBPLibary.SetDamageParamsTargetASC` _explosiondamageparams (`AbilitySystemBlueprintLibrary.GetAbilitySystemComponent` DamageTarget))
  (`AuraAbilitySystemBPLibary.ApplyDamageEffect` (`self.ExplosionDamageParams`)))

(fn `PureMakeDamageParam`
  (returns (OutOverlappingActors :type "Array of Actor Object Reference"))
  (bind _returnvalue (`self.K2_GetActorLocation`))
  (`AuraAbilitySystemBPLibary.SetDamageParamsRadialDamageOrigin` (`self.ExplosionDamageParams`) _returnvalue 66.0 100.0)
  (bind _outoverlappingactors (`AuraAbilitySystemBPLibary.GetLivePlayersWithRadius` self (`|MakeArray` self (`self.Instigator`) :!type "Actor Object Reference") _returnvalue))
  (return _outoverlappingactors))

(fn `SetApexLocation`
  (bind _returnvalue (`self.K2_GetActorLocation`))
  (set `self.BeginLocation` _returnvalue)
  (set `self.ApexLocation` (+ _returnvalue (* (`self.GetActorForwardVector`) (`self.TargetDistance`)))))

(fn `UserConstructionScript`)