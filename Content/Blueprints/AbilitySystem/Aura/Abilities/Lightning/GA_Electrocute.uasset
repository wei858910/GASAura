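; GA_Electrocute is a channeled lightning ability that fires a beam at the cursor target and chains it to additional targets.
; A montage event locks movement, adds ShockLoop cues and starts a looping timer that pays cost and deals lightning damage.
; Input release (padded to a minimum time), failed cost or primary target death ends it.
; Ending restores movement, clears cues, and applies hold-time-gated debuff damage and cooldown.
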(event `self.K2_ActivateAbility`
  (bind _charactermovement (`Character.CharacterMovement` (`self.OnwerCharacter`)))
  (if (`KismetSystemLibrary.DoesImplementInterface` (`self.GetAvatarActorFromActorInfo`) "/Script/Aura_Learn.CombatInterface")
    ;[1 1 1] 鼠标下捕获到的相关数据捕获
    (bind (_asynctaskproxy _datahandle) (`TargetDataUnderMouse.CreateTargetDataUnderMouse`)
      (:`ValidData`
        (bind _returnvalue (`AbilitySystemBlueprintLibrary.GetHitResultFromTargetData` _datahandle))
        (if (`GameplayStatics.BreakHitResult` _returnvalue)
          (`self.StoreMouseDataInfo` _returnvalue)
          (`self.StoreOnwerVaribles`)
          (`|ExecutionSequence`
            (:`then_0`
              (set `PlayerController.bShowMouseCursor` false (`self.OnwerPlayerController`))
              (message `CombatInterface.SetFaceingTargetLoc` (`self.GetAvatarActorFromActorInfo`) (`self.MouseHitLocation`))
              (`self.K2_ExecuteGameplayCue` (struct :`TagName` "GameplayCue.ShockBurst"))
              (`AbilityTask_PlayMontageAndWait.CreatePlayMontageAndWaitProxy` "None" (`self.Montage_Electrocute`)
                (:`then`
                  (`AbilityTask_WaitGameplayEvent.WaitGameplayEvent` (struct :`TagName` "Event.Montag.Electrocute") null true
                    (:`EventReceived`
                      (message `CombatInterface.SetShockLoop` (`self.GetAvatarActorFromActorInfo`) true)
                      (`MovementComponent.StopMovementImmediately` _charactermovement)
                      (`CharacterMovementComponent.DisableMovement` _charactermovement)
                      (`self.SpawnElectrocuteBeam`)
                      (bind _returnvalue_2 (`KismetSystemLibrary.K2_SetTimerDelegate` (delegate `DamageAndCost`) (`self.DamageDeltaTime`) true))
                      (set `self.DamageAndCostHandle` _returnvalue_2))))))
            (:`then_1`
              (bind (_asynctaskproxy_2 _timeheld) (`AbilityTask_WaitInputRelease.WaitInputRelease` false)
                (:`OnRelease`
                  ;[1 1 1] 太短了则要延迟结束，至少看到光束
                  (set `self.SpellTime` _timeheld)
                  (if (< (`self.SpellTime`) (`self.MinSpellTime`))
                    (`self.K2_HasAuthority`
                      (:`True`
                        (`KismetSystemLibrary.Delay` (- (`self.MinSpellTime`) (`self.SpellTime`)))
                        (`self.K2_EndAbility` :!label _label))
                      (:`False`
                        (set `PlayerController.bShowMouseCursor` true (`self.OnwerPlayerController`))))
                    (else
                      (goto _label)))))))
          (else
            (`self.K2_CancelAbility`)))))
    (else
      (`self.K2_CancelAbility`))))

(event `DamageAndCost`
  (bind _returnvalue (`self.K2_CommitAbilityCost` false))
  (if _returnvalue
    (`self.ApplayDamage`)
    (else
      (`self.K2_EndAbility`))))

(event `self.K2_OnEndAbility`
  (params (bWasCancelled :type Boolean))
  (`|ExecutionSequence`
    (:`then_0`
      (`self.ClearTimer`)
      (`self.CommitCD`))
    (:`then_1`
      (set `PlayerController.bShowMouseCursor` true (`self.OnwerPlayerController`))
      (message `CombatInterface.SetShockLoop` (`self.GetAvatarActorFromActorInfo`) false)
      (`CharacterMovementComponent.SetMovementMode` (`Character.CharacterMovement` (`self.OnwerCharacter`)) "MOVE_Walking" 0)
      ;[1 1 1] 第一个击中的是战斗对象，则移除闪电连鞭
      (if (`self.bFirstTargetCombatTarget`)
        (`GameplayCueFunctionLibrary.RemoveGameplayCueOnActor` (`self.MouseHitActor`) (struct :`TagName` "GameplayCue.ShockLoop") (`self.FirstTargetCueParams`))
        (`self.AppalyDebuffDamage` 0.5 (`self.MouseHitActor`))
        (`self.K2_HasAuthority`
          (:`True`
            ;[1 1 1] 服务器才应用伤害
            (for _array_element (`self.Additional Targets`)
              (`self.RemoveShockCueFromAddtional` _array_element)
              (`self.AppalyDebuffDamage` 1.0 _array_element)
              (`self.RemoveOnDeathNotify` _array_element)))
          (:`False`
            (for _array_element_2 (`self.Additional Targets`)
              (`self.RemoveShockCueFromAddtional` _array_element_2)
              (`self.RemoveOnDeathNotify` _array_element_2))))
        (else
          (`GameplayCueFunctionLibrary.RemoveGameplayCueOnActor` (`self.GetAvatarActorFromActorInfo`) (struct :`TagName` "GameplayCue.ShockLoop") (`self.FirstTargetCueParams`)))))
    (:`then_2`
      (`self.UnValidVaible`))))

(event `self.PrimaryTargetDied`
  (params (DeadActor :type "Actor Object Reference"))
  ;[1 1 1] 光柱的首个敌人死了直接结束
  (`GameplayCueFunctionLibrary.RemoveGameplayCueOnActor` DeadActor (struct :`TagName` "GameplayCue.ShockLoop") (`self.FirstTargetCueParams`))
  (`self.K2_EndAbility`))

(event `self.AdditionalTargetDied`
  (params (DeadActor :type "Actor Object Reference"))
  (`self.RemoveShockCueFromAddtional` DeadActor)
  (`KismetArrayLibrary.Array_RemoveItem` (`self.Additional Targets`) DeadActor)
  (`self.RemoveOnDeathNotify` DeadActor))

(fn `AddShockCueToAdditionalTarget`
  (params (AdditionalTarget :type "Actor Object Reference"))
  (locals (TargetActor :type "Actor Object Reference"))
  (bind _targetactor (`local.TargetActor`))
  (bind _returnvalue (`AbilitySystemBlueprintLibrary.MakeGameplayCueParameters` 0.0 0.0 (struct) (struct) (struct) (struct) (struct) (`Actor.K2_GetActorLocation` _targetactor) (0.0 0.0 0.0) null null _targetactor null 1 1 (`Actor.RootComponent` (`self.MouseHitActor`))))
  (bind _output_get (set `local.TargetActor` AdditionalTarget))
  (`BlueprintMapLibrary.Map_Add` (`self.AddtionalActorToCueParams`) _output_get _returnvalue)
  (`GameplayCueFunctionLibrary.AddGameplayCueOnActor` (`local.TargetActor`) (struct :`TagName` "GameplayCue.ShockLoop") _returnvalue))

(fn `AppalyDebuffDamage`
  (params (SpellTimeThreshold :type "Float (double-precision)" :default 0.5) (BeDebuffer :type "Actor Object Reference"))
  (if (> (`self.SpellTime`) SpellTimeThreshold)
    (`AuraAbilitySystemBPLibary.ApplyDamageEffect` (`self.MakeDamageEffectParamsFromClassDefaults` BeDebuffer))))

(fn `ApplayDamage`
  (locals (GESpecHandle :type "GameplayEffectSpecHandle Structure"))
  (bind _returnvalue (`self.GetAbilitySystemComponentFromActorInfo`))
  (bind _returnvalue_2 (`AbilitySystemBlueprintLibrary.GetAbilitySystemComponent` (`self.MouseHitActor`)))
  (`/Engine/EditorBlueprintResources/StandardMacros.IsValid` (`self.GetAbilitySystemComponentFromActorInfo`)
    (:`Is Valid`
      ;[1 1 1] 频率伤害只给雷伤，最后结束才给该GA的混伤+Debuff
      (bind _returnvalue_3 (`AbilitySystemBlueprintLibrary.AssignTagSetByCallerMagnitude` (`AbilitySystemComponent.MakeOutgoingSpec` _returnvalue (`self.DamageEffectClass`) (`KismetMathLibrary.Conv_IntToDouble` (`self.GetAbilityLevel`)) (`AbilitySystemComponent.MakeEffectContext` _returnvalue)) (struct :`TagName` "Damage.Lightning") (`self.GetDamageByDamageType` (`BlueprintGameplayTagLibrary.MakeLiteralGameplayTag` (struct :`TagName` "Damage.Lightning")) (`KismetMathLibrary.Conv_IntToDouble` (`self.GetAbilityLevel`)))))
      (bind _output_get (set `local.GESpecHandle` _returnvalue_3))
      (bind _returnvalue_4 (`AbilitySystemBlueprintLibrary.GetEffectContext` _output_get))
      (`AuraAbilitySystemBPLibary.SetActiveHitReact` _returnvalue_4)
      (`/Engine/EditorBlueprintResources/StandardMacros.IsValid` _returnvalue_2
        (:`Is Valid`
          (`AbilitySystemComponent.BP_ApplyGameplayEffectSpecToSelf` _returnvalue_2 _output_get))
        (:`Is Not Valid`
          _))
      (for _array_element (`self.Additional Targets`)
        (bind _returnvalue_5 (`AbilitySystemBlueprintLibrary.GetAbilitySystemComponent` _array_element))
        (`/Engine/EditorBlueprintResources/StandardMacros.IsValid` _returnvalue_5
          (:`Is Valid`
            (`AbilitySystemComponent.BP_ApplyGameplayEffectSpecToSelf` _returnvalue_5 (`local.GESpecHandle`))))))))

(fn `ClearTimer`
  (bind _damageandcosthandle (`self.DamageAndCostHandle`))
  (if (`KismetSystemLibrary.K2_IsValidTimerHandle` _damageandcosthandle)
    (`KismetSystemLibrary.K2_ClearAndInvalidateTimerHandle` _damageandcosthandle)))

(fn `CommitCD`
  (if (> (`self.SpellTime`) (`self.MinSpellTime`))
    (`self.K2_CommitAbilityCooldown` false)))

(fn `RemoveShockCueFromAddtional`
  (params (Addtional :type "Actor Object Reference"))
  (bind (_value _returnvalue) (`BlueprintMapLibrary.Map_Find` (`self.AddtionalActorToCueParams`) Addtional))
  (if _returnvalue
    (`GameplayCueFunctionLibrary.RemoveGameplayCueOnActor` Addtional (struct :`TagName` "GameplayCue.ShockLoop") _value)))

(fn `SpawnElectrocuteBeam`
  (locals (CueTarget :type "Actor Object Reference"))
  (`self.TraceFirstTarget` (`self.MouseHitLocation`))
  (bind _returnvalue (message `CombatInterface.GetWeapon` (`self.GetAvatarActorFromActorInfo`)))
  (set `self.FirstTargetCueParams` (`AbilitySystemBlueprintLibrary.MakeGameplayCueParameters` 0.0 0.0 (struct) (struct) (struct) (struct) (struct) (`self.MouseHitLocation`) (0.0 0.0 0.0) null null (`self.MouseHitActor`) null 1 1 _returnvalue))
  ;[1 1 1 1 16] 鼠标指向(已经在TarceFirst中改为第一个击中的对象)的是敌人吗？
  ; 之后如果击中敌人，则要进行闪电传递
  (bind _output_get (set `self.bFirstTargetCombatTarget` (`KismetSystemLibrary.DoesImplementInterface` (`self.MouseHitActor`) "/Script/Aura_Learn.CombatInterface")))
  (if _output_get
    (set `local.CueTarget` (`self.MouseHitActor`))
    (else
      (set `local.CueTarget` (`self.GetAvatarActorFromActorInfo`))))
  (`GameplayCueFunctionLibrary.AddGameplayCueOnActor` (`local.CueTarget`) (struct :`TagName` "GameplayCue.ShockLoop") (`self.FirstTargetCueParams`))
  (if (`self.bFirstTargetCombatTarget`)
    (bind _outadditionaltargets (`self.StoreAdditionalTargets`))
    (bind _output_get_2 (set `self.Additional Targets` _outadditionaltargets))
    (for _array_element _output_get_2
      (`self.AddShockCueToAdditionalTarget` _array_element))))

(fn `UnValidVaible`
  (`BlueprintMapLibrary.Map_Clear` (`self.AddtionalActorToCueParams`))
  (`KismetArrayLibrary.Array_Clear` (`self.Additional Targets`))
  (set `self.MouseHitActor` null)
  (set `self.bFirstTargetCombatTarget` false)
  (set `self.SpellTime` 0.0))