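; Gameplay ability that casts a Fire Bolt toward the point under the mouse.
; Valid target data sets the avatar's facing location through CombatInterface, then starts the cast montage.
; A montage gameplay event triggers SpawnProjectile at the stored target location.
; EndAbility is left unwired, with a note that ending immediately on the server keeps clients from receiving the ability trigger.
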(event `self.K2_ActivateAbility`
  (bind (_asynctaskproxy _datahandle) (`TargetDataUnderMouse.CreateTargetDataUnderMouse` self)
    (:`ValidData`
      (bind (_returnvalue_bblockinghit _returnvalue_binitialoverlap _returnvalue_time _returnvalue_distance _returnvalue_location) (`GameplayStatics.BreakHitResult` (`AbilitySystemBlueprintLibrary.GetHitResultFromTargetData` _datahandle)))
      (set `self.ProjectileTargetLoc` _returnvalue_location)
      (bind _ascombat_interface (cast `CombatInterface` (`self.GetAvatarActorFromActorInfo`)))
      (`CombatInterface.SetFaceingTargetLoc` _ascombat_interface (`self.ProjectileTargetLoc`))
      (`AbilityTask_PlayMontageAndWait.CreatePlayMontageAndWaitProxy` "None" "/Game/Assets/Characters/Aura/Animations/Abilities/AM_Cast_FireBolt.AM_Cast_FireBolt"
        (:`then`
          (`AbilityTask_WaitGameplayEvent.WaitGameplayEvent` (struct :`TagName` "Event.Montag.FireBolt") null
            (:`EventReceived`
              (`self.SpawnProjectile` (`self.ProjectileTargetLoc`)))))))))