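; BP_EnemyBase is a base enemy character Blueprint that supplies spawn, dissolve and facing effects.
; After parent BeginPlay, a timeline animates actor scale for a bouncy pop-in.
; Two events run separate timelines that drive the "Dissolve" scalar on dynamic material instances passed in for mesh and weapon.
; Another event writes a given location into the "FacingTarget" Motion Warping target, so warped animations can face it.
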(event `self.ReceiveBeginPlay`
  (`parent.ReceiveBeginPlay`)
  ;[1 1 1] 通过缩放模型营造弹跳感
  (bind (_direction _scalvalue) (`Timeline|ScalPop`)
    (:`Update`
      (`self.SetActorScale3D` (`KismetMathLibrary.Conv_DoubleToVector` _scalvalue)))))

(event `self.ReceiveTick`
  (params (DeltaSeconds :type "Float (single-precision)")))

(event `self.StartDissolveTimlineOfMesh`
  (params (DynamicMaterialInstance :type "MaterialInstanceDynamic Object Reference"))
  (bind (_direction _dissolve) (`Timeline|DissolveTimelineOfMesh`)
    (:`Update`
      (`MaterialInstanceDynamic.SetScalarParameterValue` DynamicMaterialInstance "Dissolve" _dissolve))))

(event `self.StartDissolveTimlineOfWeapon`
  (params (DynamicMaterialInstance :type "MaterialInstanceDynamic Object Reference"))
  (bind (_direction _dissolve) (`Timeline|DissolveTimelineOfWeapon`)
    (:`Update`
      (`MaterialInstanceDynamic.SetScalarParameterValue` DynamicMaterialInstance "Dissolve" _dissolve))))

(event `CombatInterface.SetFaceingTargetLoc`
  (params (FaceingLoction :type "Vector Structure (by ref)"))
  (`MotionWarpingComponent.AddOrUpdateWarpTargetFromLocation` (`self.MotionWarping`) "FacingTarget" FaceingLoction))

(fn `UserConstructionScript`)